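; Enemy mortar turret that calls FireAnyway every tick and shows a world-space health bar.
; On BeginPlay it hands itself to the health bar widget and caches the player's tank pawn.
; Each tick it rotates the widget component toward the player's camera, then destroys that component once HealthComponent's current health reaches zero.
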(event EventBeginPlay
  (bind _asw_hp_bar_enemy_turret_mortire (Utilities|Casting|CastToW_HpBar_EnemyTurret_Mortire (UserInterface|GetUserWidgetObject (Variables|Default|GetWidget%20Heaalth))))
  (Variables|/Game/Widgets/HP/W_HpBar_EnemyTurret_Mortire.W_HpBar_EnemyTurret_Mortire_C|SetEnemyTurret%20Mortire _asw_hp_bar_enemy_turret_mortire self)
  (bind _asbp_tank_pawn (Utilities|Casting|CastToBP_TankPawn (Game|Player|GetPlayerPawn 0)))
  (Variables|Default|SetPlayer _asbp_tank_pawn))

(event Collision|EventActorBeginOverlap
  (params (OtherActor :type Actor%20Object%20Reference)))

(event EventTick
  (params (DeltaSeconds :type Float%20%28single-precision%29))
  (bind _widget_heaalth (Variables|Default|GetWidget%20Heaalth))
  (bind _player (Variables|Default|GetPlayer))
  (bind _returnvalue (Transformation|GetWorldLocation _widget_heaalth))
  (bind _cameracomponent (Variables|/Script/TankProject.TankPawn|GetCameraComponent _player))
  (bind _returnvalue_2 (Transformation|GetWorldLocation _cameracomponent))
  (Class|Turret|FireAnyway)
  (if (Utilities|IsValid (Variables|Default|GetWidget%20Heaalth))
    (Transformation|SetWorldRotation _widget_heaalth (Math|Rotator|FindLookatRotation (Math|Vector|MakeVector (.x _returnvalue) (.y _returnvalue) 0.0) (Math|Vector|MakeVector (.x _returnvalue_2) (.y _returnvalue_2) 0.0)) false false)
    (if (== (Variables|/Script/TankProject.HealthComponent|GetCurrentHealth (Variables|Default|GetHealthComponent)) 0.0)
      (Components|DestroyComponent (Variables|Default|GetWidget%20Heaalth)))))

(fn ConstructionScript)