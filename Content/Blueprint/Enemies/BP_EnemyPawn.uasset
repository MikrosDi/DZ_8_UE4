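; Enemy tank pawn Blueprint that manages a floating health bar above the enemy.
; On BeginPlay it hands itself to the W_HpBar_EnemyTank widget and caches the player's BP_TankPawn.
; Each tick it turns the widget toward the player using only X and Y positions, keeping it level, and destroys it when HealthComponent health reaches zero.
; A FireAnyway call is left unconnected and never runs.
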(event EventBeginPlay
  (bind _asw_hp_bar_enemy_tank (Utilities|Casting|CastToW_HpBar_EnemyTank (UserInterface|GetUserWidgetObject (Variables|Default|GetWidget%20Health))))
  (Variables|/Game/Widgets/HP/W_HpBar_EnemyTank.W_HpBar_EnemyTank_C|SetEnemyTank _asw_hp_bar_enemy_tank self)
  (bind _asbp_tank_pawn (Utilities|Casting|CastToBP_TankPawn (Game|Player|GetPlayerPawn 0)))
  (Variables|Default|SetPlayer _asbp_tank_pawn))

(event Collision|EventActorBeginOverlap
  (params (OtherActor :type Actor%20Object%20Reference)))

(event EventTick
  (params (DeltaSeconds :type Float%20%28single-precision%29))
  (bind _widget_health (Variables|Default|GetWidget%20Health))
  (bind _player (Variables|Default|GetPlayer))
  (bind _returnvalue (Transformation|GetWorldLocation _widget_health))
  (bind _rootcomponent (Variables|/Script/Engine.Actor|GetRootComponent _player))
  (bind _returnvalue_2 (Transformation|GetWorldLocation _rootcomponent))
  (if (Utilities|IsValid (Variables|Default|GetWidget%20Health))
    (Transformation|SetWorldRotation _widget_health (Math|Rotator|FindLookatRotation (Math|Vector|MakeVector (.x _returnvalue) (.y _returnvalue) 0.0) (Math|Vector|MakeVector (.x _returnvalue_2) (.y _returnvalue_2) 0.0)) false false)
    (if (== (Variables|/Script/TankProject.HealthComponent|GetCurrentHealth (Variables|Default|GetHealthComponent)) 0.0)
      (Components|DestroyComponent (Variables|Default|GetWidget%20Health)))))

(fn ConstructionScript)